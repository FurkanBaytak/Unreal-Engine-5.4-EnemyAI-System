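; Base enemy Blueprint that provides a sword attack and a sword-wielding action.
; WieldSword spawns BP_Sword, snaps it to the right-hand socket and sets the wielding flag.
; Attack plays a slash montage and fires the attack-end dispatcher on completion or interruption.
; ChasePlayer, an early Blueprint copy of BT_Enemy_Base's chase noted as non-working, loops move-to-player, attack and delay, with no caller in this graph.
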(event Custom|ChasePlayer
  ;[1 1 1] BT_Enemy_Base kovalama işleminin aynısının blueprint olarak ilk deneyimleri, bu kod şu anda çalışmıyor.
  (AI|AIMoveTo self "0, 0, 0" (Game|GetPlayerCharacter 0) 1.5e+02 false
    (:OnSuccess
      (CallFunction|Attack)
      (Utilities|FlowControl|Delay 2.0)
      (CallFunction|ChasePlayer))))

(event Custom|Attack
  (Animation|Montage|PlayMontage (Variables|Character|GetMesh) "/Game/Animations/Montage_Sword_Slash.Montage_Sword_Slash"
    (:OnCompleted
      _)
    (:OnInterrupted
      _))
  (Default|CallOnAtackEnd))

(event Custom|WieldSword
  (bind _returnvalue (Game|SpawnActorfromClass "/Game/Weapons/BP_Sword.BP_Sword_C" (Transformation|GetActorTransform) "Undefined" "MultiplyWithRoot" 0 0))
  (Transformation|AttachComponentToComponent _returnvalue (Variables|Character|GetMesh) "hand_r_sword_socket" "SnapToTarget" "SnapToTarget" "SnapToTarget" true)
  (Variables|Default|SetIsWeildingSword true))

(event EventBeginPlay)

(fn ConstructionScript)